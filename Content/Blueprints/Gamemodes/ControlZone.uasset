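; ControlZone is a capture zone actor that switches ownership between Team Red and Team Blue.
; Begin and end overlaps update the occupant list and run CheckTeam, which compares occupants against the first player controller's team to detect contested zones.
; A successful check restarts the TeamProgress timeline, while a failed one stops it.
; When the timeline finishes, the zone takes the new team and shows that team's cylinder mesh.
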(event EventBeginPlay
  (Variables|Default|SetcurrentTeam "NewEnumerator0")
  (Variables|Default|SetteamConflicted false))

(event Collision|EventActorBeginOverlap
  (params (OtherActor :type Actor%20Object%20Reference))
  (bind _teamtoswitch (Variables|Default|GetTeamToSwitch))
  (Utilities|Array|AddUnique (Variables|Default|GetentityWithin) OtherActor)
  (Variables|Default|SetlastEntity OtherActor)
  (Development|PrintString "LETS GO")
  (bind _startswitch (CallFunction|CheckTeam))
  (if _startswitch
    (Timeline|Team%20Progress PlayFromStart
      (:Finished
        (Variables|Default|SetcurrentTeam _teamtoswitch)
        (switch Utilities|FlowControl|Switch|SwitchonTeams _teamtoswitch
          (:NewEnumerator1
            (Rendering|SetVisibility (Variables|Default|GetCylinder) false false)
            (Rendering|SetVisibility (Variables|Default|GetCylinder1) true false)
            (Rendering|SetVisibility (Variables|Default|GetCylinder2) false false))
          (:NewEnumerator2
            (Rendering|SetVisibility (Variables|Default|GetCylinder) false false)
            (Rendering|SetVisibility (Variables|Default|GetCylinder1) false false)
            (Rendering|SetVisibility (Variables|Default|GetCylinder2) true false)))))
    (else
      (Timeline|Team%20Progress Stop))))

(event EventTick
  (params (DeltaSeconds :type Float%20%28single-precision%29)))

(event Collision|EventActorEndOverlap
  (params (OtherActor :type Actor%20Object%20Reference))
  (bind _teamtoswitch (Variables|Default|GetTeamToSwitch))
  (Utilities|Array|RemoveItem (Variables|Default|GetentityWithin) OtherActor)
  (bind _startswitch (CallFunction|CheckTeam))
  (if _startswitch
    (Timeline|Team%20Progress PlayFromStart
      (:Finished
        (Variables|Default|SetcurrentTeam _teamtoswitch)
        (switch Utilities|FlowControl|Switch|SwitchonTeams _teamtoswitch
          (:NewEnumerator1
            (Rendering|SetVisibility (Variables|Default|GetCylinder) false false)
            (Rendering|SetVisibility (Variables|Default|GetCylinder1) true false)
            (Rendering|SetVisibility (Variables|Default|GetCylinder2) false false))
          (:NewEnumerator2
            (Rendering|SetVisibility (Variables|Default|GetCylinder) false false)
            (Rendering|SetVisibility (Variables|Default|GetCylinder1) false false)
            (Rendering|SetVisibility (Variables|Default|GetCylinder2) true false)))))
    (else
      (Timeline|Team%20Progress Stop))))

(fn ConstructionScript)

(fn CheckTeam
  (bind _entitywithin (Variables|Default|GetentityWithin))
  (bind _returnvalue (Utilities|Array|Length _entitywithin))
  (bind _team (Class|InterfaceTeam|GetTeam(Message) (Game|GetPlayerController 0)))
  (if (== _returnvalue 0)
    (return false)
    (elif (> _returnvalue 1)
      (bind _array_element (Utilities|Array|ForEachLoopwithBreak _entitywithin :!label _label)
        (:LoopBody
          (bind _team_2 (Class|InterfaceTeam|GetTeam(Message) _array_element))
          (if (Utilities|Enum|Equal(Enum) _team_2 _team)
            (Variables|Default|SetteamConflicted false)
            (else
              (Variables|Default|SetteamConflicted true)
              (goto _label Break))))
        (:Completed
          (if (Variables|Default|GetteamConflicted)
            _
            (elif (Utilities|Enum|Equal(Enum) _team (Variables|Default|GetcurrentTeam))
              _
              (else
                (Variables|Default|SetTeamToSwitch _team :!label _label_2)
                (return true))))
          (return false)))
      (else
        (goto _label_2)))))